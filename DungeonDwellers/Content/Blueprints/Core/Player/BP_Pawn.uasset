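; BP_Pawn is a player camera pawn that pans along world X and Y and zooms through a spring arm.
; Forward and side axis inputs shift a target location, while the zoom axis adjusts a clamped target arm length.
; Tick interpolates the actor location and spring arm length toward those targets for smooth movement, without sweeping for collision.
; Panning steps are added per input call without delta-time scaling.
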(event EventTick
  (params (DeltaSeconds :type Float%20%28single-precision%29))
  (bind _springarm (Variables|Default|GetSpringArm))
  (Variables|/Script/Engine.SpringArmComponent|SetTargetArmLength _springarm (Math|Interpolation|FInterpTo (Variables|/Script/Engine.SpringArmComponent|GetTargetArmLength _springarm) (Variables|Default|GetZoomDes) DeltaSeconds 2.0))
  (Transformation|SetActorLocation (Math|Interpolation|VInterpTo (Transformation|GetActorLocation) (Variables|Default|GetLocationDes) DeltaSeconds 5.0) false false))

(event EventBeginPlay
  (Variables|Default|SetLocationDes (Transformation|GetActorLocation))
  (Variables|Default|SetZoomDes (Variables|/Script/Engine.SpringArmComponent|GetTargetArmLength (Variables|Default|GetSpringArm))))

(event Input|AxisEvents|InputAxisInputAxis_Zoom
  (params (AxisValue :type Float%20%28single-precision%29))
  (Variables|Default|SetZoomDes (Math|Float|Clamp(Float) (+ (* AxisValue 5e+01) (Variables|Default|GetZoomDes)) 1e+02 2.5e+03)))

(event Input|AxisEvents|InputAxisInputAxis_Forward
  (params (AxisValue :type Float%20%28single-precision%29))
  (Variables|Default|SetLocationDes (+ (Variables|Default|GetLocationDes) (Math|Vector|MakeVector (* AxisValue 2e+01) 0.0 0.0))))

(event Input|AxisEvents|InputAxisInputAxis_Side
  (params (AxisValue :type Float%20%28single-precision%29))
  (Variables|Default|SetLocationDes (+ (Variables|Default|GetLocationDes) (Math|Vector|MakeVector 0.0 (* AxisValue 2e+01) 0.0))))

(fn ConstructionScript)